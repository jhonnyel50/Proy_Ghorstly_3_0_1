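; Paper2D side-view character (alma-A) that walks along world Y and opens level "nivel2" when clicked.
; The DERECHA axis turns the sprite to face the input direction and adds movement input.
; Each axis event also refreshes the flipbook through ControlDeAnimaciones from falling and moving states.
; That selection is unfinished: every branch picks the same index, the options are empty and the Idle, Run and Jump flipbook variables are unused.
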(event Custom|Animaciones
  (Variables|Default|SetenMovimiento (> (Math|Vector|VectorLength (Transformation|GetVelocity)) 0.0))
  (Variables|Default|SetenCaida (AI|Components|NavMovement|IsFalling (Variables|Character|GetCharacterMovement)))
  (bind _salifdaflipbook (CallFunction|ControlDeAnimaciones (Variables|Default|GetenCaida) (Variables|Default|GetenMovimiento)))
  (Sprite|SetFlipbook (Variables|Default|GetSprite) _salifdaflipbook))

(event EventBeginPlay)

(event MouseInput|EventActorOnClicked
  (params (ButtonPressed :type Key%20Structure :default "None"))
  (Game|OpenLevel(byName) "nivel2"))

(event EventTick
  (params (DeltaSeconds :type Float%20%28single-precision%29)))

(event Input|AxisEvents|InputAxisDERECHA
  (params (AxisValue :type Float%20%28single-precision%29))
  (bind _sprite (Variables|Default|GetSprite))
  (CallFunction|Animaciones)
  (if (> AxisValue 0.0)
    (Transformation|SetRelativeRotation _sprite "0,180.000000, 0" false false)
    (Pawn|Input|AddMovementInput "0.000000,1.000000, 0" AxisValue false :!label _label)
    (elif (< AxisValue 0.0)
      (Transformation|SetRelativeRotation _sprite "0, 0, 0" false false)
      (goto _label))))

(fn ConstructionScript)

(fn ControlDeAnimaciones
  (params (EnCaida :type Boolean) (EnMovimientp :type Boolean))
  (LocalVariables|SetcaidaLocal EnCaida)
  (LocalVariables|SetmovimientoLocal EnMovimientp)
  (if (LocalVariables|GetcaidaLocal)
    (LocalVariables|SetanimacionesD 0)
    (elif (LocalVariables|GetmovimientoLocal)
      (LocalVariables|SetanimacionesD 0)
      (else
        (LocalVariables|SetanimacionesD 0))))
  (return (Utilities|Select :Index (LocalVariables|GetanimacionesD) :Option%200 0 :Option%201 0 :Option%202 0)))