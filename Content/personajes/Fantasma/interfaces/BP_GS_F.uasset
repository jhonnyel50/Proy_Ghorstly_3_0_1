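; Game State for the Fantasma game mode that holds a match time limit and runs a server-side match timer.
; On BeginPlay, the authority starts a one-shot 30-second timer and copies TiempoMaximo from GM_fantasma.
; When the timer fires, it only prints a debug message if ElapsedTime is within that limit.
; The player controller call to switch to "nivel_2" is disconnected, and the construction script just assigns TiempoMaximo to itself.
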(event Custom|tiepo%20partida
  (if (>= (Variables|Default|Gettiempo%20maximo) (Variables|Default|GetElapsedTime))
    (Development|PrintString "iniciando" true true "(R=0.000000,G=1.000000,B=0.033423,A=1.000000)")))

(event EventBeginPlay
  (Networking|SwitchHasAuthority
    (:Authority
      (Utilities|Time|SetTimerbyEvent (delegate Custom|tiepo%20partida) 3e+01)
      (bind _asgm_fantasma (Utilities|Casting|CastToGM_fantasma (Game|GetGameMode)))
      (Variables|Default|Settiempo%20maximo (Variables|/Game/personajes/Fantasma/interfaces/GM_fantasma.GM_fantasma_C|Gettiempo%20maximo _asgm_fantasma)))))

(event EventTick
  (params (DeltaSeconds :type Float%20%28single-precision%29)))

(fn ConstructionScript
  (Networking|SwitchHasAuthority
    (:Authority
      (Utilities|Casting|CastToGameMode (Game|GetGameMode))
      (Variables|Default|Settiempo%20maximo (Variables|Default|Gettiempo%20maximo)))))