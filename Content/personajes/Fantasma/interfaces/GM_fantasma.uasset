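; GM_fantasma is a game mode Blueprint that tracks joining players and broadcasts countdown and chat events to them.
; PostLogin adds each BP_PC_F controller to PlayersF, stores the returned index in ConteoPlayers and copies the array to the game instance's Personajes.
; The countdown event shows the countdown on every controller, guarded by a started flag, while mensajes relays chat to all.
; View-target and BP_fantasma spawn nodes are left unconnected.
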(event Custom|coutdown
  (if (not (Variables|Default|Getstrarted))
    (for _array_element (Variables|Default|GetPlayers_F)
      (Variables|Default|Setstrarted true)
      (Default|Showcoutdown _array_element))))

(event Custom|mensajes
  (params (NewParam :type String) (NewParam2 :type String))
  ;[1 1 1] chat
  (for _array_element (Variables|Default|GetPlayers_F)
    (Default|Mensajesplayers _array_element NewParam NewParam2)))

(event EventBeginPlay)

(event EventTick
  (params (DeltaSeconds :type Float%20%28single-precision%29)))

(event EventPostLogin
  (params (NewPlayer :type Player%20Controller%20Object%20Reference))
  (bind _asbp_pc_f (Utilities|Casting|CastToBP_PC_F NewPlayer))
  (bind _returnvalue (Utilities|Array|Add (Variables|Default|GetPlayers_F) _asbp_pc_f))
  (Variables|Default|Setconteo%20players _returnvalue)
  (bind _asgame_instancia (Utilities|Casting|CastTogame-instancia (Game|GetGameInstance)))
  (Variables|/Game/Blueprints/online/instance/game-instancia.game-instancia_C|Setpersonajes _asgame_instancia (Variables|Default|GetPlayers_F)))

(fn ConstructionScript)