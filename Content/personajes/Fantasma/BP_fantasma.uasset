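; Playable ghost (Fantasma) character for a 2D side-scroller, with X-axis movement, jumping and velocity-based sprite flipping.
; BeginPlay adds Enhanced Input, authority-dependent keyboard widgets and a player HUD, then calls the game instance's ghost camera function.
; Keys open the pause menu or toggle the HUD's player display, which Tick also drives from Pulsado.
; The almitas event shows a fire, water, earth or wind widget by flag, clearing that flag after a delay.
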(event Custom|mostrar-jugadores
  (bind _widged_jugador (Variables|Default|Getwidged%20jugador))
  ;[1 1 1] interfaces para el juego
  (if (Variables|Default|Getpulsado)
    (Default|MostrarJugadores _widged_jugador true)
    (else
      (Default|MostrarJugadores _widged_jugador false))))

(event Custom|almitas
  (bind _returnvalue (Game|GetPlayerController 0))
  (bind _returnvalue_2 (Game|GetPlayerController 0))
  (bind _returnvalue_3 (Game|GetPlayerController 0))
  (bind _returnvalue_4 (Game|GetPlayerController 0))
  (Utilities|FlowControl|Sequence
    (:then_0
      ;[1 1 1] interfaces para el juego
      (if (Variables|Default|Getfueguito)
        (bind _returnvalue_5 (UserInterface|CreateWidget "/Game/Blueprints/interfaces-alma/interfaz-fuego.interfaz-fuego_C" _returnvalue))
        (UserInterface|Viewport|AddtoViewport _returnvalue_5 0)
        (Input|SetInputModeUIOnly _returnvalue 0 "DoNotLock" false)
        (Variables|/Script/Engine.PlayerController|SetbShowMouseCursor _returnvalue true)
        (Input|SetInputModeGameOnly _returnvalue false)
        (Utilities|FlowControl|Delay 3.0)
        (Variables|Booleanos|SetFueguito false)
        (elif (Variables|Default|Getaguita)
          (bind _returnvalue_6 (UserInterface|CreateWidget "/Game/Blueprints/interfaces-alma/interfaz-agua.interfaz-agua_C" _returnvalue_2))
          (UserInterface|Viewport|AddtoViewport _returnvalue_6 0)
          (Input|SetInputModeUIOnly _returnvalue_2 0 "DoNotLock" false)
          (Variables|/Script/Engine.PlayerController|SetbShowMouseCursor _returnvalue_2 true)
          (Input|SetInputModeGameOnly _returnvalue_2 false)
          (Utilities|FlowControl|Delay 3.0)
          (Variables|Booleanos|SetAguita false)
          (elif (Variables|Default|Gettierrita)
            (bind _returnvalue_7 (UserInterface|CreateWidget "/Game/Blueprints/interfaces-alma/interfaz-tierra.interfaz-tierra_C" _returnvalue_3))
            (UserInterface|Viewport|AddtoViewport _returnvalue_7 0)
            (Input|SetInputModeUIOnly _returnvalue_3 0 "DoNotLock" false)
            (Variables|/Script/Engine.PlayerController|SetbShowMouseCursor _returnvalue_3 true)
            (Input|SetInputModeGameOnly _returnvalue_3 false)
            (Utilities|FlowControl|Delay 3.0)
            (Variables|Booleanos|SetTierrita false)
            (elif (Variables|Default|Getvientito)
              (bind _returnvalue_8 (UserInterface|CreateWidget "/Game/Blueprints/interfaces-alma/interfaz-viento.interfaz-viento_C" _returnvalue_4))
              (UserInterface|Viewport|AddtoViewport _returnvalue_8 0)
              (Input|SetInputModeUIOnly _returnvalue_4 0 "DoNotLock" false)
              (Variables|/Script/Engine.PlayerController|SetbShowMouseCursor _returnvalue_4 true)
              (Input|SetInputModeGameOnly _returnvalue_4 false)
              (Utilities|FlowControl|Delay 3.0)
              (Variables|Booleanos|SetVientito false))))))))

(event Custom|Movimiento_F
  (params (NewParam :type Float%20%28double-precision%29))
  ;[1 1 1] Movimiento
  (Pawn|Input|AddMovementInput "1.000000,0.000000,0.000000" NewParam false))

(event Input|EnhancedActionEvents|EnhancedInputActionINP_jump
  (params (ActionValue :type Boolean) (ElapsedSeconds :type Float%20%28double-precision%29) (TriggeredSeconds :type Float%20%28double-precision%29) (InputAction :type Input%20Action%20Object%20Reference :default "/Game/Blueprints/Inputs/Action/INP_jump.INP_jump"))
  ;[1 1 1] Movimiento
  (:Started
    (Character|Jump)))

(event Input|EnhancedActionEvents|EnhancedInputActionINP_move
  (params (ActionValue :type Float%20%28double-precision%29) (ElapsedSeconds :type Float%20%28double-precision%29) (TriggeredSeconds :type Float%20%28double-precision%29) (InputAction :type Input%20Action%20Object%20Reference :default "/Game/Blueprints/Inputs/Action/INP_move.INP_move"))
  ;[1 1 1] Movimiento
  (Pawn|Input|AddMovementInput "1.000000,0.000000,0.000000" ActionValue false))

(event EventBeginPlay
  (bind _returnvalue (Game|GetPlayerController 0))
  (Utilities|FlowControl|Sequence
    (:then_0
      ;[1 1 1] Movimiento
      (CallFunction|AddPlayerInput))
    (:then_1
      ;[1 1 1] interfaces para el juego
      (Networking|SwitchHasAuthority
        (:Authority
          (bind _returnvalue_2 (UserInterface|CreateWidget "/Game/Blueprints/interfaz-personajes/Fantasma/Teclado_F.Teclado_F_C" _returnvalue))
          (UserInterface|Viewport|AddtoViewport _returnvalue_2 0))
        (:Remote
          (bind _returnvalue_3 (UserInterface|CreateWidget "/Game/Blueprints/interfaz-personajes/Fantasma/Teclado_F1.Teclado_F1_C" _returnvalue))
          (UserInterface|Viewport|AddtoViewport _returnvalue_3 0))))
    (:then_2
      (bind _returnvalue_4 (UserInterface|CreateWidget "/Game/personajes/Fantasma/interfaces/online/BP_Hud_F.BP_Hud_F_C" _returnvalue (Variables|Default|Getplayer%20state)))
      (bind _output_get (Variables|Default|Setwidged%20jugador _returnvalue_4))
      (UserInterface|Viewport|AddtoViewport _output_get 0))
    (:then_3
      (bind _asgame_instancia (Utilities|Casting|CastTogame-instancia (Game|GetGameInstance)))
      (Default|CamaraF _asgame_instancia (Game|GetPlayerController 0)))))

(event EventTick
  (params (DeltaSeconds :type Float%20%28single-precision%29))
  (bind _widged_jugador (Variables|Default|Getwidged%20jugador))
  (bind _sprite (Variables|Default|GetSprite))
  (Utilities|FlowControl|Sequence
    (:then_0
      ;[1 1 1] rotacion
      (Math|Float|CompareFloat (.x (Transformation|GetVelocity)) 0.0
        (:>
          (Transformation|SetRelativeRotation _sprite (Math|Rotator|MakeRotator 0.0 0.0 1.8e+02) false false))
        (:<
          (Transformation|SetRelativeRotation _sprite (Math|Rotator|MakeRotator 0.0 0.0 0.0) false false))))
    (:then_1
      ;[1 1 1] interfaces para el juego
      (if (Variables|Default|Getpulsado)
        (Default|MostrarJugadores _widged_jugador true)
        (else
          (Default|MostrarJugadores _widged_jugador false))))))

(event Collision|EventActorBeginOverlap
  (params (OtherActor :type Actor%20Object%20Reference))
  ;[1 1 1] interfaces para el juego
)

(event Input|ActionEvents|InputActionatake
  (params (Key :type Key%20Structure :default "None")))

(event Input|AxisEvents|InputAxisDERECHA
  (params (AxisValue :type Float%20%28single-precision%29))
  ;[1 1 1] Movimiento
  (Pawn|Input|AddMovementInput "1.000000,0.000000,0.000000" (stale Custom|Movimiento_F NewParam) false))

(event Input|KeyboardEvents|2
  (params (Key :type Key%20Structure :default "None"))
  (bind _returnvalue (Game|GetPlayerController 0))
  (:Pressed
    (bind _returnvalue_2 (UserInterface|CreateWidget "/Game/Blueprints/Interfaces_juego/menu-pausa.menu-pausa_C" _returnvalue))
    (UserInterface|Viewport|AddtoViewport _returnvalue_2 0)
    (Variables|/Script/Engine.PlayerController|SetbShowMouseCursor _returnvalue true)))

(event Input|KeyboardEvents|3
  (params (Key :type Key%20Structure :default "None"))
  (bind _widged_jugador (Variables|Default|Getwidged%20jugador))
  (:Pressed
    ;[1 1 1] interfaces para el juego
    (Default|MostrarJugadores _widged_jugador true))
  (:Released
    (Default|MostrarJugadores _widged_jugador false)))

(fn ConstructionScript)

(fn ControlDeAnimaciones
  (params (enCaida :type Boolean) (Enmovimineto :type Boolean) (NewParam1 :type Float%20%28double-precision%29))
  (bind _sprite (Variables|Default|GetSprite))
  (if (> NewParam1 0.0)
    (Transformation|SetRelativeRotation _sprite "0, 0, 0" false false)
    (if Enmovimineto :!label _label
      (LocalVariables|SetAnimaciones%20D "NewEnumerator1")
      (else
        (LocalVariables|SetAnimaciones%20D "NewEnumerator0")))
    (return (Utilities|Select :Index (LocalVariables|GetAnimaciones%20D) :NewEnumerator0 (Variables|Default|GetidleFlipbook) :NewEnumerator1 (Variables|Default|GetrunnFlipbook) :NewEnumerator2 0 :NewEnumerator3 0 :NewEnumerator4 0))
    (elif (< NewParam1 0.0)
      (Transformation|SetRelativeRotation _sprite "0.000000,180.000000,0.000000" false false)
      (goto _label))))

(fn AddPlayerInput
  (bind _asplayer_controller (Utilities|Casting|CastToPlayerController (Pawn|GetController)))
  (Input|AddMappingContext (PlayerController|LocalPlayerSubsystems|GetEnhancedInputLocalPlayerSubsystem _asplayer_controller) "/Game/Blueprints/Inputs/IMC_action.IMC_action" 0 "(bIgnoreAllPressedKeysUntilRelease=True,bForceImmediately=False,bNotifyUserSettings=False)"))

(fn Rotacion
  (bind _sprite (Variables|Default|GetSprite))
  ;[1 1 1] rotacion
  (Math|Float|CompareFloat (.x (Transformation|GetVelocity)) 0.0
    (:>
      (Transformation|SetRelativeRotation _sprite (Math|Rotator|MakeRotator 0.0 0.0 1.8e+02) false false))
    (:<
      (Transformation|SetRelativeRotation _sprite (Math|Rotator|MakeRotator 0.0 0.0 0.0) false false))))