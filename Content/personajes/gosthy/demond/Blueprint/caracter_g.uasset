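; Paper2D player character for the ghosty, with sideways movement, footstep sound and HUD widgets created at BeginPlay.
; Movement flips the flipbook by direction, and ControlDeAnimaciones picks its animation from velocity, falling state and input.
; Key 2 opens the pause menu, while key 3 and a Tick check on Pulsado toggle the HUD player list.
; The almitas event opens fire, water, earth or wind widgets from element flags; their removal chains are unconnected.
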(event Custom|mostrar-jugadores
  (bind _widged_jugador (Variables|Default|Getwidged%20jugador))
  ;[1 1 1] interfaces para el juego
  (if (Variables|Default|Getpulsado)
    (Default|MostrarJugadores _widged_jugador true)
    (else
      (Default|MostrarJugadores _widged_jugador false))))

(event Custom|almitas
  (bind _returnvalue (Game|GetPlayerController 0))
  (bind _returnvalue_2 (Game|GetPlayerController 0))
  (bind _returnvalue_3 (Game|GetPlayerController 0))
  (bind _returnvalue_4 (Game|GetPlayerController 0))
  (Utilities|FlowControl|Sequence
    (:then_0
      ;[1 1 1] interfaces para el juego
      (if (Variables|Default|Getfueguito)
        (bind _returnvalue_5 (UserInterface|CreateWidget "/Game/Blueprints/interfaces-alma/interfaz-fuego.interfaz-fuego_C" _returnvalue))
        (UserInterface|Viewport|AddtoViewport _returnvalue_5 0)
        (Input|SetInputModeUIOnly _returnvalue 0 "DoNotLock" false)
        (Variables|/Script/Engine.PlayerController|SetbShowMouseCursor _returnvalue true)
        (Input|SetInputModeGameOnly _returnvalue false)))
    (:then_1
      (if (Variables|Default|Getaguita)
        (bind _returnvalue_6 (UserInterface|CreateWidget "/Game/Blueprints/interfaces-alma/interfaz-agua.interfaz-agua_C" _returnvalue_2))
        (UserInterface|Viewport|AddtoViewport _returnvalue_6 0)
        (Input|SetInputModeUIOnly _returnvalue_2 0 "DoNotLock" false)
        (Variables|/Script/Engine.PlayerController|SetbShowMouseCursor _returnvalue_2 true)
        (Input|SetInputModeGameOnly _returnvalue_2 false)))
    (:then_2
      (if (Variables|Default|Gettierrita)
        (bind _returnvalue_7 (UserInterface|CreateWidget "/Game/Blueprints/interfaces-alma/interfaz-tierra.interfaz-tierra_C" _returnvalue_3))
        (UserInterface|Viewport|AddtoViewport _returnvalue_7 0)
        (Input|SetInputModeUIOnly _returnvalue_3 0 "DoNotLock" false)
        (Variables|/Script/Engine.PlayerController|SetbShowMouseCursor _returnvalue_3 true)
        (Input|SetInputModeGameOnly _returnvalue_3 false)))
    (:then_3
      (if (Variables|Default|Getvientito)
        (bind _returnvalue_8 (UserInterface|CreateWidget "/Game/Blueprints/interfaces-alma/interfaz-viento.interfaz-viento_C" _returnvalue_4))
        (UserInterface|Viewport|AddtoViewport _returnvalue_8 0)
        (Input|SetInputModeUIOnly _returnvalue_4 0 "DoNotLock" false)
        (Variables|/Script/Engine.PlayerController|SetbShowMouseCursor _returnvalue_4 true)
        (Input|SetInputModeGameOnly _returnvalue_4 false)))))

(event Custom|animaciones
  (params (NewParam :type Float%20%28double-precision%29))
  (bind _returnvalue (Transformation|GetVelocity))
  (bind _returnvalue_2 (Math|Vector|VectorLength _returnvalue))
  ;[1 1 1] control de animaciones
  (Variables|Character|SetEnMovimiento (== _returnvalue_2 0.0))
  (Variables|Character|SetEnMovimiento (> _returnvalue_2 0.0))
  (Variables|Default|SetEnCaida (AI|Components|NavMovement|IsFalling (Variables|Character|GetCharacterMovement)))
  (bind _flip (CallFunction|ControlDeAnimaciones (Variables|Default|GetEnCaida) (Variables|Character|GetEnMovimiento) NewParam))
  (Sprite|SetFlipbook (Variables|Default|GetPaperFlipbook) _flip))

(event Custom|movimiento
  (params (NewParam :type Float%20%28double-precision%29))
  (bind _paperflipbook (Variables|Default|GetPaperFlipbook))
  ;[1 1 1] movimiento de personaje
  (if (> NewParam 0.0)
    (Transformation|SetRelativeRotation _paperflipbook "0,180.000000, 0" false false)
    (Pawn|Input|AddMovementInput "0.000000,1.000000,10000.000000" NewParam false :!label _label)
    (if (not (AI|Components|NavMovement|IsFalling (Variables|Character|GetCharacterMovement)))
      (Utilities|FlowControl|Delay 0.2)
      (Audio|PlaySoundatLocation 0 (Transformation|GetWorldLocation (Variables|Collision|GetCapsuleComponent)) "0, 0, 0" 1.0 1.0 0.0 0 0 0 0))
    (elif (< NewParam 0.0)
      (Transformation|SetRelativeRotation _paperflipbook "0, 0, 0" false false)
      (goto _label))))

(event EventBeginPlay
  (Utilities|FlowControl|Sequence
    (:then_0
      ;[1 1 1] interfaces para el juego
      (bind _returnvalue (UserInterface|CreateWidget "/Game/Blueprints/interfaz-personajes/teclado-ghosty1.teclado-ghosty1_C" (Game|GetPlayerController 0)))
      (UserInterface|Viewport|AddtoViewport _returnvalue 0))
    (:then_1
      (bind _returnvalue_2 (UserInterface|CreateWidget "/Game/Blueprints/online/personajes/bp-hud.bp-hud_C" (Game|GetPlayerController 0) (Variables|Default|Getplayer%20state)))
      (bind _output_get (Variables|Default|Setwidged%20jugador _returnvalue_2))
      (UserInterface|Viewport|AddtoViewport _output_get 0))))

(event EventTick
  (params (DeltaSeconds :type Float%20%28single-precision%29))
  (bind _widged_jugador (Variables|Default|Getwidged%20jugador))
  ;[1 1 1] interfaces para el juego
  (if (Variables|Default|Getpulsado)
    (Default|MostrarJugadores _widged_jugador true)
    (else
      (Default|MostrarJugadores _widged_jugador false))))

(event Input|ActionEvents|InputActionatake
  (params (Key :type Key%20Structure :default "None")))

(event Input|AxisEvents|InputAxisDERECHA
  (params (AxisValue :type Float%20%28single-precision%29))
  (bind _paperflipbook (Variables|Default|GetPaperFlipbook))
  ;[1 1 1] movimiento de personaje
  (if (> (stale Custom|movimiento NewParam) 0.0)
    (Transformation|SetRelativeRotation _paperflipbook "0,180.000000, 0" false false)
    (Pawn|Input|AddMovementInput "0.000000,1.000000,10000.000000" (stale Custom|movimiento NewParam) false :!label _label)
    (if (not (AI|Components|NavMovement|IsFalling (Variables|Character|GetCharacterMovement)))
      (Utilities|FlowControl|Delay 0.2)
      (Audio|PlaySoundatLocation 0 (Transformation|GetWorldLocation (Variables|Collision|GetCapsuleComponent)) "0, 0, 0" 1.0 1.0 0.0 0 0 0 0))
    (elif (< (stale Custom|movimiento NewParam) 0.0)
      (Transformation|SetRelativeRotation _paperflipbook "0, 0, 0" false false)
      (goto _label))))

(event Input|KeyboardEvents|2
  (params (Key :type Key%20Structure :default "None"))
  (bind _returnvalue (Game|GetPlayerController 0))
  ;[1 1 1] interfaces para el juego
  (:Pressed
    (bind _returnvalue_2 (UserInterface|CreateWidget "/Game/Blueprints/Interfaces_juego/menu-pausa.menu-pausa_C" _returnvalue))
    (UserInterface|Viewport|AddtoViewport _returnvalue_2 0)
    (Variables|/Script/Engine.PlayerController|SetbShowMouseCursor _returnvalue true)))

(event Input|KeyboardEvents|3
  (params (Key :type Key%20Structure :default "None"))
  (bind _widged_jugador (Variables|Default|Getwidged%20jugador))
  ;[1 1 1] interfaces para el juego
  (:Pressed
    (Default|MostrarJugadores _widged_jugador true))
  (:Released
    (Default|MostrarJugadores _widged_jugador false)))

(fn ConstructionScript)

(fn ControlDeAnimaciones
  (params (enCaida :type Boolean) (Enmovimineto :type Boolean) (NewParam1 :type Float%20%28double-precision%29))
  (bind _paperflipbook (Variables|Default|GetPaperFlipbook))
  (LocalVariables|SetCaida%20Local enCaida)
  (LocalVariables|SetMovimiento%20Local Enmovimineto)
  (if (> NewParam1 0.0)
    (Transformation|SetRelativeRotation _paperflipbook "0,180.000000, 0" false false)
    (if (LocalVariables|GetMovimiento%20Local) :!label _label
      (LocalVariables|Setanimaciones%20D "NewEnumerator1")
      (else
        (LocalVariables|Setanimaciones%20D "NewEnumerator0" :!label _label_2)))
    (elif (< NewParam1 0.0)
      (Transformation|SetRelativeRotation _paperflipbook "0, 0, 0" false false)
      (if (LocalVariables|GetCaida%20Local)
        (LocalVariables|Setanimaciones%20D "NewEnumerator0")
        (else
          (goto _label)))
      (else
        (goto _label_2))))
  (return (Utilities|Select :Index (LocalVariables|Getanimaciones%20D) :Option%200 (Variables|Default|GetjumpFlipbook) :Option%201 (Variables|Default|GetidleFlipbook) :Option%202 (Variables|Default|GetrunnFlipbook) :Option%203 0)))