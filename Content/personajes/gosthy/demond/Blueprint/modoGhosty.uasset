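; Game mode for the Ghosty mode that tracks joining players and relays countdown and chat events to them.
; PostLogin casts each new controller to the custom player-controller and adds it to a Players array.
; The countdown event calls Showcoutdown on every player while Strarted is false, and the mensajes event forwards two chat parameters to each player.
; Setting Strarted and spawning Caracter_g at indexed player starts exist only as disconnected, unused logic.
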(event Custom|coutdown
  (if (not (Variables|Default|Getstrarted))
    (for _array_element (Variables|Default|Getplayers)
      (Default|Showcoutdown _array_element))))

(event Custom|mensajes
  (params (NewParam :type String) (NewParam2 :type String))
  ;[1 1 1] chat
  (for _array_element (Variables|Default|Getplayers)
    (Default|Mensajesplayers _array_element NewParam NewParam2)))

(event EventBeginPlay)

(event EventTick
  (params (DeltaSeconds :type Float%20%28single-precision%29)))

(event EventPostLogin
  (params (NewPlayer :type Player%20Controller%20Object%20Reference))
  (bind _asplayer_controller (Utilities|Casting|CastToplayer-controller NewPlayer))
  (Utilities|Array|Add (Variables|Default|Getplayers) _asplayer_controller))

(fn ConstructionScript)